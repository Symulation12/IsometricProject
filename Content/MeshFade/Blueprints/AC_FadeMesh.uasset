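; Actor component that fades the owner's first static mesh in and out by temporarily swapping its materials for fade versions.
; BeginFade creates and caches dynamic instances of FadeMaterials, applies them, then enables tick; EndFade reverses the fade.
; Tick stands in for a timeline, moving the eased "Fade" parameter until either end is reached, then switching itself off.
; Original materials, saved at BeginPlay, are restored once the fade fully reverses.
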(event EventBeginPlay
  (CallFunction|SetupFade))

(event EventTick
  (params (DeltaSeconds :type Float%20%28single-precision%29))
  (CallFunction|UpdateFade DeltaSeconds))

(fn UpdateFade
  (params (DeltaTime :type Float%20%28single-precision%29))
  (Variables|Default|SetFadeCurrent (Math|Interpolation|FInterptoConstant (Variables|Default|GetFadeCurrent) (Math|Float|SelectFloat 1.0 0.0 (Variables|Default|GetbFadeActive)) DeltaTime (Variables|Default|GetFadeInterpSpeed)))
  (for _array_element (Variables|Default|GetDMI_FadeList)
    (Rendering|Material|SetScalarParameterValue _array_element "Fade" (Class|KismetMathLibrary|FInterpEaseinOut 0.0 (Variables|Default|GetFadeMax) (Variables|Default|GetFadeCurrent) 2.0) :!class /Script/Engine.MaterialInstanceDynamic))
  (if (Variables|Default|GetbFadeActive)
    (if (>= (Variables|Default|GetFadeCurrent) 1.0)
      (Components|Tick|SetComponentTickEnabled false) ; DONE - STOP TICK FOR NOW
    )
    (elif (<= (Variables|Default|GetFadeCurrent) 0.0)
      (Components|Tick|SetComponentTickEnabled false) ; DONE - STOP TICK FOR NOW
      (CallFunction|SetDefaultMaterials) ; RESET MATERIALS
    )))

(fn BeginFade
  (Utilities|IsValid (Variables|Default|GetMesh) ; If we have a mesh
    (:Is%20Valid
      (if (> (Utilities|Array|Length (Variables|Default|GetFadeMaterials)) 0) ; If we have materials
        (if (> (Utilities|Array|Length (Variables|Default|GetDMI_FadeList)) 0) ; Create Dynamic Mat Instances if needed
          _
          (else
            (for _array_element (Variables|Default|GetFadeMaterials) ; Use the desired versions of our fade materials
              (bind _returnvalue (Rendering|Material|CreateDynamicMaterialInstance _array_element "None" "None" :!class /Script/Engine.KismetMaterialLibrary))
              (Utilities|Array|Add (Variables|Default|GetDMI_FadeList) _returnvalue))))
        (for (_array_element_2 _array_index) (Variables|Default|GetDMI_FadeList) ; Swap materials to DMI
          (Rendering|Material|SetMaterial (Variables|Default|GetMesh) _array_index _array_element_2))
        (Variables|Default|SetbFadeActive true)
        (Components|Tick|SetComponentTickEnabled true) ; Only tick when we need to update\nActor components have no timeline, otherwise we'd use that
      ))))

(fn SetupFade
  (Variables|Default|SetMesh (Actor|GetComponentbyClass (Components|GetOwner) "/Script/Engine.StaticMeshComponent"))
  (bind _mesh (Variables|Default|GetMesh) ; Save Defaults
    (:then
      (Variables|Default|SetDefaultMaterials (Rendering|Material|GetMaterials _mesh)))
    (:else)))

(fn EndFade
  (Utilities|IsValid (Variables|Default|GetMesh) ; If we have a mesh
    (:Is%20Valid
      (if (> (Utilities|Array|Length (Variables|Default|GetDefaultMaterials)) 0) ; If we have materials
        (if (> (Utilities|Array|Length (Variables|Default|GetDMI_FadeList)) 0) ; If we have DMI
          (Variables|Default|SetbFadeActive false) ; Set false to reverse
          (Components|Tick|SetComponentTickEnabled true))))))

(fn SetDefaultMaterials
  (Utilities|IsValid (Variables|Default|GetMesh)
    (:Is%20Valid
      (if (> (Utilities|Array|Length (Variables|Default|GetDefaultMaterials)) 0)
        (for (_array_element _array_index) (Variables|Default|GetDefaultMaterials)
          (Rendering|Material|SetMaterial (Variables|Default|GetMesh) _array_index _array_element))))))
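; Pawn component that fades meshes blocking the view between the player camera and its pawn.
; Each tick it sphere-traces from camera toward pawn, stopping a radius short to skip actors behind the player.
; An optional second trace, offset by clamped velocity, catches obstructions ahead of movement.
; Hit actors' AC_FadeMesh components are diffed against the current list, calling BeginFade on new entries and EndFade on dropped ones.
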(event EventBeginPlay
  (CallFunction|SetupFadeController))

(event EventTick
  (params (DeltaSeconds :type Float%20%28single-precision%29))
  (CallFunction|UpdateFadeComponent DeltaSeconds))

(fn CheckFadeMeshes
  (params (DeltaTime :type Float%20%28single-precision%29))
  (bind _pawn (Variables|Default|GetPawn)
    (:then
      (bind _camera (Variables|Default|GetCamera)
        (:then
          (LocalVariables|SetStart (Camera|GetCameraLocation _camera))
          (LocalVariables|SetEnd (Transformation|GetActorLocation _pawn))
          (LocalVariables|SetVel (Transformation|GetVelocity _pawn))
          (LocalVariables|SetEnd (+ (LocalVariables|GetEnd) (* (Math|Vector|GetUnitDirection(Vector) (LocalVariables|GetEnd) (LocalVariables|GetStart)) (Variables|Default|GetFadeRadius)))) ; Remove radius distance from\nour end point so we don't overlap\nactors behind the player - Just between\ncamera and player
          (Utilities|FlowControl|Sequence
            (:then_0
              (bind _outhits (Collision|MultiSphereTraceByChannel (LocalVariables|GetStart) (LocalVariables|GetEnd) (Variables|Default|GetFadeRadius) "TraceTypeQuery3" false (Utilities|Array|MakeArray (Variables|Default|GetPawn)) "None" true "(R=1.000000,G=0.000000,B=0.000000,A=1.000000)" "(R=0.000000,G=1.000000,B=0.000000,A=1.000000)" DeltaTime)) ; CURRENT
              (for _array_element _outhits
                (Utilities|IsValid (Actor|GetComponentbyClass (.HitActor (Collision|BreakHitResult _array_element)) "/Game/MeshFade/Blueprints/AC_FadeMesh.AC_FadeMesh_C")
                  (:Is%20Valid
                    (Utilities|Array|Add (LocalVariables|GetFadeComponents) (Actor|GetComponentbyClass (.HitActor (Collision|BreakHitResult _array_element)) "/Game/MeshFade/Blueprints/AC_FadeMesh.AC_FadeMesh_C"))))))
            (:then_1
              (if (CallFunction|ShouldCheckVelocityFade (LocalVariables|GetVel))
                (bind _outhits_2 (Collision|MultiSphereTraceByChannel (+ (LocalVariables|GetStart) (Math|Vector|ClampVectorSize (* (LocalVariables|GetVel) (Variables|Default|GetVelocityMultiplier)) 0.0 (Variables|Default|GetVelocityMax))) (+ (LocalVariables|GetEnd) (Math|Vector|ClampVectorSize (* (LocalVariables|GetVel) (Variables|Default|GetVelocityMultiplier)) 0.0 (Variables|Default|GetVelocityMax))) (Variables|Default|GetFadeRadius) "TraceTypeQuery3" false (Utilities|Array|MakeArray (Variables|Default|GetPawn)) "None" true "(R=1.000000,G=0.000000,B=0.000000,A=1.000000)" "(R=0.000000,G=1.000000,B=0.000000,A=1.000000)" DeltaTime)) ; VELOCITY LOCATION
                (for _array_element_2 _outhits_2
                  (Utilities|IsValid (Actor|GetComponentbyClass (.HitActor (Collision|BreakHitResult _array_element_2)) "/Game/MeshFade/Blueprints/AC_FadeMesh.AC_FadeMesh_C")
                    (:Is%20Valid
                      (Utilities|Array|Add (LocalVariables|GetFadeComponents) (Actor|GetComponentbyClass (.HitActor (Collision|BreakHitResult _array_element_2)) "/Game/MeshFade/Blueprints/AC_FadeMesh.AC_FadeMesh_C")))))))
            (:then_2
              (return (LocalVariables|GetFadeComponents)))))
        (:else)))
    (:else)))

(fn UpdateFadeComponent
  (params (DeltaTime :type Float%20%28single-precision%29))
  (bind _fadelist (CallFunction|CheckFadeMeshes DeltaTime))
  (LocalVariables|SetDesiredList _fadelist)
  (LocalVariables|SetCurrentList (Variables|Default|GetFadeMeshCurrentList)) ; Save current list so when we\nremove or add items we don't\nscrew up the for each loops
  (if (not (Utilities|Array|Identical (LocalVariables|GetDesiredList) (LocalVariables|GetCurrentList))) ; IF SAME - SKIP
    (Utilities|FlowControl|Sequence
      (:then_0
        (for _array_element (LocalVariables|GetCurrentList) ; REMOVE MISSING
          (LocalVariables|SetMesh _array_element)
          (if (not (Utilities|Array|ContainsItem (LocalVariables|GetDesiredList) (LocalVariables|GetMesh)))
            (Default|EndFade (LocalVariables|GetMesh))
            (Utilities|Array|RemoveItem (Variables|Default|GetFadeMeshCurrentList) (LocalVariables|GetMesh)))))
      (:then_1
        (for _array_element_2 (LocalVariables|GetDesiredList) ; ADD NEW
          (LocalVariables|SetMesh _array_element_2)
          (if (not (Utilities|Array|ContainsItem (Variables|Default|GetFadeMeshCurrentList) (LocalVariables|GetMesh)))
            (Default|BeginFade (LocalVariables|GetMesh))
            (Utilities|Array|Add (Variables|Default|GetFadeMeshCurrentList) (LocalVariables|GetMesh))))))))

(fn SetupFadeController
  (bind _aspawn (Utilities|Casting|CastToPawn (Components|GetOwner)))
  (bind _output_get (Variables|Default|SetPawn _aspawn))
  (bind _asplayer_controller (Utilities|Casting|CastToPlayerController (Pawn|GetController _output_get)))
  (bind _playercameramanager (Variables|/Script/Engine.PlayerController|GetPlayerCameraManager _asplayer_controller)
    (:then
      (Variables|Default|SetCamera _playercameramanager))
    (:else)))

(fn ShouldCheckVelocityFade
  (params (Velocity :type Vector))
  (return (and (Variables|Default|GetbCheckVelocity) (> (Math|Vector|VectorLengthSquared Velocity) 0.0))))